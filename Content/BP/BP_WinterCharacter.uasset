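; Player character for a winter survival game, managing health, food, arrows, experience and leveling.
; A one-second looping timer started on possession drains food, then damages or heals the character per the IsDamage flag set by TickDamage/TickRecovery.
; Experience pickups also add extra food; level-ups load max stats from StateDataTable and level up the BP_Tent.
; Empty food or health triggers GameOver, which only prints and stops the timer.
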(event `self.ReceiveBeginPlay`
  (`parent.ReceiveBeginPlay`)
  (add `self.m_OnTakeExp` (delegate `TakeExp`)))

(event `TakeExp` :!signature `self.m_OnTakeExp`
  (params (amount :type "Float (double-precision)"))
  (set `self.Exp` (+ amount (`self.Exp`)))
  (`self.CheckExp`)
  (`self.AddFood`))

(event `self.ReceivePossessed`
  (params (NewController :type "Controller Object Reference"))
  (`parent.ReceivePossessed` NewController)
  (`self.InitState`)
  (`self.CreateUI`)
  (`self.StartTick`)
  (bind _outactors (`GameplayStatics.GetAllActorsOfClass` "/Game/BP/BP_Tent.BP_Tent_C"))
  (for _array_element _outactors
    (set `self.Tent` _array_element))
  (`AudioComponent.Play` (`self.Audio`) 0.0))

(event `/Game/BP/BP_Winter_Interface.InitExpNumber`
  (set `self.Exp` 0.0))

(event `StartTick`
  (bind _returnvalue (`KismetSystemLibrary.K2_SetTimerDelegate` (delegate `TickTimeEvent`) 1.0 true))
  (set `self.TickTime` _returnvalue))

(event `TickTimeEvent`
  (bind _bissurvival (`self.CheckFood`))
  (if _bissurvival
    (if (`self.bIsDamage`)
      (`GameplayStatics.ApplyDamage` self 1.0)
      (else
        (`self.RecoveryHP` (`self.GetTentRecovery`))))
    (else
      (`self.GameOver`))))

(event `self.ReceiveAnyDamage`
  (params (Damage :type "Float (single-precision)") (DamageType :type "DamageType Object Reference") (InstigatedBy :type "Controller Object Reference") (DamageCauser :type "Actor Object Reference"))
  (bind _returnvalue (- (`self.GetCurHP`) Damage))
  (if (> _returnvalue 0.0)
    (`self.SetCurHP` _returnvalue)
    (else
      (`self.SetCurHP` 0.0)
      (`self.GameOver`))))

(event `/Game/BP/BP_Winter_Interface.TickRecovery`
  (set `self.bIsDamage` false)
  (`self.RecoverArrowCount`)
  (`self.RecoveryFoodGauge`))

(event `GameOver`
  (`KismetSystemLibrary.PrintString` "GameOver" true true (struct :`G` 0.66 :`B` 1.0 :`A` 1.0) 10.0)
  (`KismetSystemLibrary.K2_ClearAndInvalidateTimerHandle` (`self.TickTime`)))

(event `/Game/BP/BP_Winter_Interface.TickDamage`
  (set `self.bIsDamage` true))

(fn `AddFood`
  (`self.SetExtrafood` (+ (`self.GetExtrafood`) 1)))

(fn `CheckExp`
  (if (>= (`self.GetCurExp`) (`self.GetMaxExp`))
    (`self.Level Up`)))

(fn `CheckFood`
  (returns (bIsSurvival :type Boolean))
  (if (`self.bIsDamage`)
    (bind _newparam (`self.CheckFoodGauge`))
    (return _newparam)
    (elif (> (`self.GetExtrafood`) 0)
      (`self.SetExtrafood` (- (`self.GetExtrafood`) 1))
      (return true)
      (else
        (bind _newparam_2 (`self.CheckFoodGauge`))
        (return _newparam_2)))))

(fn `CheckFoodGauge`
  (returns (NewParam :type Boolean))
  (`self.SetCurFoodGauge` (- (`self.GetCurFoodGauge`) 1.0))
  (if (> (`self.GetCurFoodGauge`) 0.0)
    (return true)
    (else
      (`self.SetCurFoodGauge` 0.0)
      (return false))))

(fn `CreateUI`
  (bind _returnvalue (`|CreateWidget` "/Game/BP/Widgets/BP_StateUI.BP_StateUI_C" (`GameplayStatics.GetPlayerController` 0)))
  (`UserWidget.AddToViewport` _returnvalue 0))

(fn `GetArrowNumber`
  (returns (ArrowNumber :type Integer))
  (return (`self.GetArrowCrnCount`)))

(fn `GetCurExp`
  (returns (Exp :type "Float (double-precision)"))
  (return (`self.Exp`)))

(fn `GetCurFoodGauge`
  (returns (FoodGauge :type "Float (double-precision)"))
  (return (`self.CurFoodGauge`)))

(fn `GetCurHP`
  (returns (HP :type "Float (double-precision)"))
  (return (`self.m_fCrnHealth`)))

(fn `GetExpNumber`
  (returns (ExpNumber :type "Float (double-precision)"))
  (return (`self.Exp`)))

(fn `GetExtrafood`
  (returns (Food :type Integer))
  (return (`self.Extrafood`)))

(fn `GetMaxArrowNumber`
  (returns (ArrowNumber :type Integer))
  (return (`self.MaxArrowNumber`)))

(fn `GetMaxExp`
  (returns (Exp :type "Float (double-precision)"))
  (return (`self.MaxExp`)))

(fn `GetMaxFoodGauge`
  (returns (FoodGauge :type "Float (double-precision)"))
  (return (`self.MaxFoodGauge`)))

(fn `GetMaxHP`
  (returns (HP :type "Float (double-precision)"))
  (return (`self.m_fHealth`)))

(fn `GetStateTable`
  (params (RowName :type Name))
  (returns (MaxHP :type "Float (double-precision)") (MaxExp :type "Float (double-precision)") (ArrowNumber :type Integer))
  (bind _returnvalue (`|GetDataTableRow` "/Game/BP/DateTable/StateDataTable.StateDataTable" RowName)
    (:`then`
      (bind (_maxhp _maxexp _arrownumber) (break `/Game/BP/Structure/BP_State` _returnvalue))
      (return _maxhp _maxexp _arrownumber))))

(fn `GetTentRecovery`
  (returns (NewParam :type "Float (double-precision)"))
  (return (* (`self.GetMaxHP`) 0.2)))

(fn `InitState`
  (bind (_maxhp _maxexp _arrownumber) (`self.GetStateTable` "1"))
  (`self.InitBow` _arrownumber)
  (set `self.m_fHealth` _maxhp)
  (set `self.MaxExp` _maxexp)
  (`self.SetCurHP` (`self.GetMaxHP`))
  (`self.SetCurFoodGauge` (`self.GetMaxFoodGauge`)))

(fn `Level Up`
  (bind _tent (`self.Tent`))
  (bind (_maxhp _maxexp _arrownumber) (`self.GetStateTable` (`KismetStringLibrary.Conv_StringToName` (`KismetStringLibrary.Conv_IntToString` (`self.Level`)))))
  (`/Engine/EditorBlueprintResources/StandardMacros.IncrementInt` (`self.Level`)
    (:`  `
      (`self.SetMaxState` _maxhp _maxexp _arrownumber)
      (`self.SetCurExp` 0.0)
      (`/Engine/EditorBlueprintResources/StandardMacros.IsValid` _tent
        (:`Is Valid`
          (`/Game/BP/BP_Tent.LevelUp` _tent (- (`self.Level`) 2)))))))

(fn `RecoveryFoodGauge`
  (locals (NewLocalVar_0 :type Integer :default 0))
  (bind _foodgauge (`self.GetMaxFoodGauge`))
  (if (< (`self.GetCurFoodGauge`) (`self.GetMaxFoodGauge`))
    (`self.SetCurFoodGauge` (+ (`self.GetCurFoodGauge`) (`KismetMathLibrary.Conv_IntToDouble` (`self.GetExtrafood`))))
    (if (> (`self.GetCurFoodGauge`) (`self.GetMaxFoodGauge`))
      (`self.SetExtrafood` (`KismetMathLibrary.FTrunc` (- (`self.GetCurFoodGauge`) _foodgauge)))
      (`self.SetCurFoodGauge` _foodgauge)
      (else
        (`self.SetExtrafood` 0)))))

(fn `RecoveryHP`
  (params (NewParam :type "Float (double-precision)"))
  (bind _returnvalue (+ NewParam (`self.GetCurHP`)))
  (`self.SetCurHP` (select `bool` (< _returnvalue (`self.GetMaxHP`)) :`false` (`self.GetMaxHP`) :`true` _returnvalue)))

(fn `SetCurExp`
  (params (Exp :type "Float (double-precision)"))
  (set `self.Exp` Exp))

(fn `SetCurFoodGauge`
  (params (CurFoodGauge :type "Float (double-precision)"))
  (set `self.CurFoodGauge` CurFoodGauge))

(fn `SetCurHP`
  (params (HP :type "Float (double-precision)"))
  (set `self.m_fCrnHealth` HP))

(fn `SetExtrafood`
  (params (Food :type Integer))
  (set `self.Extrafood` Food))

(fn `SetMaxState`
  (params (MaxHP :type "Float (double-precision)") (MaxExp :type "Float (double-precision)") (MaxArrowNumber :type Integer))
  (set `self.m_fHealth` MaxHP)
  (set `self.MaxExp` MaxExp)
  (`self.SetArrowMaxCount` MaxArrowNumber))

(fn `UserConstructionScript`
  (`parent.UserConstructionScript`))