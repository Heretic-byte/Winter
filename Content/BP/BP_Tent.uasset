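; BP_Tent is a tent that sends overlapping actors a recovery message when they enter its Cone and a damage message when they leave.
; It also accumulates experience, loading MaxExp from a data table row at BeginPlay.
; SetExp resets Exp to zero on reaching MaxExp, discarding overflow, and calls LevelUp.
; LevelUp is currently empty, as its nodes for loading the next table row are disconnected.
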(event `self.ReceiveBeginPlay`
  (`self.SetMaxExp` "2")
  (set `self.NextTableNum` 3))

(event `self.Cone.OnComponentBeginOverlap`
  (params (OverlappedComponent :type "PrimitiveComponent Object Reference") (OtherActor :type "Actor Object Reference") (OtherComp :type "PrimitiveComponent Object Reference") (OtherBodyIndex :type Integer) (bFromSweep :type Boolean) (SweepResult :type "HitResult Structure (by ref)"))
  (message `/Game/BP/BP_Winter_Interface.TickRecovery` OtherActor))

(event `self.Cone.OnComponentEndOverlap`
  (params (OverlappedComponent :type "PrimitiveComponent Object Reference") (OtherActor :type "Actor Object Reference") (OtherComp :type "PrimitiveComponent Object Reference") (OtherBodyIndex :type Integer))
  (message `/Game/BP/BP_Winter_Interface.TickDamage` OtherActor))

(fn `LevelUp`)

(fn `SetExp`
  (params (NewParam :type Integer))
  (bind _returnvalue (+ NewParam (`self.Exp`)))
  (if (<= (`self.MaxExp`) _returnvalue)
    (`KismetSystemLibrary.PrintString` (`KismetStringLibrary.Concat_StrStr` "Exp : " (`KismetStringLibrary.Conv_IntToString` (`self.Exp`)) " , MaxExp : " (`KismetStringLibrary.Conv_IntToString` (`self.MaxExp`))))
    (set `self.Exp` 0)
    (`self.LevelUp`)
    (else
      (set `self.Exp` _returnvalue))))

(fn `SetMaxExp`
  (params (RowName :type Name))
  (bind _returnvalue (`|GetDataTableRow` "/Game/BP/DateTable/ExpDataTable.ExpDataTable" RowName)
    (:`then`
      (set `self.MaxExp` (`.MaxExp_8_63B15BE34ECCCB6DEA4142843F58196E` (break `/Game/BP/Structure/BP_Exp` _returnvalue))))))

(fn `UserConstructionScript`)