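; BP_ExpTest is an experience pickup that grants Exp to an actor overlapping its Box.
; On BeginPlay, SetType takes a random index to choose the mesh shape and Exp value, though RandomInteger(2) never selects the Cube tier.
; The overlap sends Exp through SetExpNumberMessage to the other actor, and a true return disables Box collision and destroys the pickup.
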(event `self.ReceiveBeginPlay`
  (`self.SetType` (`KismetMathLibrary.RandomInteger` 2)))

(event `self.Box.OnComponentBeginOverlap`
  (params (OverlappedComponent :type "PrimitiveComponent Object Reference") (OtherActor :type "Actor Object Reference") (OtherComp :type "PrimitiveComponent Object Reference") (OtherBodyIndex :type Integer) (bFromSweep :type Boolean) (SweepResult :type "HitResult Structure (by ref)"))
  (bind _bisactive (message `/Game/BP/BP_Winter_Interface.SetExpNumber` OtherActor (`self.Exp`)))
  (if _bisactive
    (`PrimitiveComponent.SetCollisionEnabled` (`self.Box`) "NoCollision")
    (`self.K2_DestroyActor`)))

(fn `SetType`
  (params (NewParam :type Integer))
  (bind _mesh (`self.Mesh`))
  (switch `int` NewParam
    (:`Default`
      (`StaticMeshComponent.SetStaticMesh` _mesh "/Engine/BasicShapes/Sphere.Sphere" :!label _label)
      (set `self.Exp` 1))
    (:`0`
      (goto _label))
    (:`1`
      (`StaticMeshComponent.SetStaticMesh` _mesh "/Engine/BasicShapes/Cylinder.Cylinder")
      (set `self.Exp` 2))
    (:`2`
      (`StaticMeshComponent.SetStaticMesh` _mesh "/Engine/BasicShapes/Cube.Cube")
      (set `self.Exp` 3))))

(fn `UserConstructionScript`)