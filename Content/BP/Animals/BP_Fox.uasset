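; BP_Fox is the fox animal Blueprint, and its only logic handles the animal's sounds.
; AttackSound, DeathSound and HowlSound events each stop the shared MSoundComp audio component, swap in their clip and play it from the start, cutting off any sound already playing on it.
; All three clips are wolf audio assets, while BeginPlay, overlap, Tick and the construction script are empty.
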(event `AttackSound`
  (bind _m_soundcomp (`self.m_SoundComp`))
  (`AudioComponent.Stop` _m_soundcomp)
  (set `AudioComponent.Sound` "/Game/Audio/Audio_Wolf_Barking.Audio_Wolf_Barking" _m_soundcomp)
  (`AudioComponent.Play` _m_soundcomp 0.0))

(event `DeathSound`
  (bind _m_soundcomp (`self.m_SoundComp`))
  (`AudioComponent.Stop` _m_soundcomp)
  (set `AudioComponent.Sound` "/Game/Audio/Audio_Wolf_Die.Audio_Wolf_Die" _m_soundcomp)
  (`AudioComponent.Play` _m_soundcomp 0.0))

(event `HowlSound`
  (bind _m_soundcomp (`self.m_SoundComp`))
  (`AudioComponent.Stop` (`self.m_SoundComp`))
  (set `AudioComponent.Sound` "/Game/Audio/Wolf_Howl.Wolf_Howl" _m_soundcomp)
  (`AudioComponent.Play` _m_soundcomp 0.0))

(fn `UserConstructionScript`)